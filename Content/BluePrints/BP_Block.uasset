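; Track block that randomly dresses four obstacle slots and has the game mode add another block when the player character overlaps its trigger, then destroys itself.
; On BeginPlay, each slot has a coin-flip chance of a random sidewalk (1, 4) or street (2, 3) mesh.
; Tick slides the street obstacles along world -Y by a fixed, frame-rate-dependent step.
; The player character hitting any obstacle quits the game.
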(event `self.ReceiveBeginPlay`
  (`self.SpawnObstacles`))

(event `self.ReceiveTick`
  (params (DeltaSeconds :type "Float (single-precision)"))
  (`self.Move Car` (`self.Obstacle2`))
  (`self.Move Car` (`self.Obstacle3`)))

(event `self.overlap.OnComponentBeginOverlap`
  (params (OverlappedComponent :type "PrimitiveComponent Object Reference") (OtherActor :type "Actor Object Reference") (OtherComp :type "PrimitiveComponent Object Reference") (OtherBodyIndex :type Integer) (bFromSweep :type Boolean) (SweepResult :type "HitResult Structure (by ref)"))
  (cast `/Game/ThirdPerson/Blueprints/BP_ThirdPersonCharacter` OtherActor)
  (bind _asbp_third_person_game_mode (cast `/Game/ThirdPerson/Blueprints/BP_ThirdPersonGameMode` (`GameplayStatics.GetGameMode`)))
  (`/Game/ThirdPerson/Blueprints/BP_ThirdPersonGameMode.Add Block` _asbp_third_person_game_mode)
  (`self.K2_DestroyActor`))

(event `self.Obstacle1.OnComponentHit`
  (params (HitComponent :type "PrimitiveComponent Object Reference") (OtherActor :type "Actor Object Reference") (OtherComp :type "PrimitiveComponent Object Reference") (NormalImpulse :type "Vector Structure") (Hit :type "HitResult Structure (by ref)"))
  (cast `/Game/ThirdPerson/Blueprints/BP_ThirdPersonCharacter` OtherActor)
  (`KismetSystemLibrary.QuitGame` null "Quit"))

(event `self.Obstacle2.OnComponentHit`
  (params (HitComponent :type "PrimitiveComponent Object Reference") (OtherActor :type "Actor Object Reference") (OtherComp :type "PrimitiveComponent Object Reference") (NormalImpulse :type "Vector Structure") (Hit :type "HitResult Structure (by ref)"))
  (cast `/Game/ThirdPerson/Blueprints/BP_ThirdPersonCharacter` OtherActor)
  (`KismetSystemLibrary.QuitGame` null "Quit"))

(event `self.Obstacle3.OnComponentHit`
  (params (HitComponent :type "PrimitiveComponent Object Reference") (OtherActor :type "Actor Object Reference") (OtherComp :type "PrimitiveComponent Object Reference") (NormalImpulse :type "Vector Structure") (Hit :type "HitResult Structure (by ref)"))
  (cast `/Game/ThirdPerson/Blueprints/BP_ThirdPersonCharacter` OtherActor)
  (`KismetSystemLibrary.QuitGame` null "Quit"))

(event `self.Obstacle4.OnComponentHit`
  (params (HitComponent :type "PrimitiveComponent Object Reference") (OtherActor :type "Actor Object Reference") (OtherComp :type "PrimitiveComponent Object Reference") (NormalImpulse :type "Vector Structure") (Hit :type "HitResult Structure (by ref)"))
  (cast `/Game/ThirdPerson/Blueprints/BP_ThirdPersonCharacter` OtherActor)
  (`KismetSystemLibrary.QuitGame` null "Quit"))

(fn `Move Car`
  (params (MeshPlaceholder :type "StaticMeshComponent Object Reference"))
  (`SceneComponent.K2_SetWorldLocation` MeshPlaceholder (+ (`SceneComponent.K2_GetComponentLocation` MeshPlaceholder) (* (0.0 -1.0 0.0) 10.0)) false false))

(fn `SpawnObstacles`
  (bind _outitem (`KismetArrayLibrary.Array_Random` (`self.SidewalkMeshes`)))
  (bind _outitem_2 (`KismetArrayLibrary.Array_Random` (`self.StreetMeshes`)))
  (bind _returnvalue (`KismetMathLibrary.Conv_IntToBool` (`KismetMathLibrary.RandomIntegerInRange` 0 1)))
  (bind _returnvalue_2 (`KismetMathLibrary.Conv_IntToBool` (`KismetMathLibrary.RandomIntegerInRange` 0 1)))
  (bind _returnvalue_3 (`KismetMathLibrary.Conv_IntToBool` (`KismetMathLibrary.RandomIntegerInRange` 0 1)))
  (bind _returnvalue_4 (`KismetMathLibrary.Conv_IntToBool` (`KismetMathLibrary.RandomIntegerInRange` 0 1)))
  (`|ExecutionSequence`
    (:`then_0`
      (`KismetSystemLibrary.PrintString` (`KismetStringLibrary.Conv_BoolToString` _returnvalue_4))
      (if _returnvalue_4
        (`StaticMeshComponent.SetStaticMesh` (`self.Obstacle1`) _outitem)))
    (:`then_1`
      (`KismetSystemLibrary.PrintString` (`KismetStringLibrary.Conv_BoolToString` _returnvalue))
      (if _returnvalue
        (`StaticMeshComponent.SetStaticMesh` (`self.Obstacle2`) _outitem_2)))
    (:`then_2`
      (`KismetSystemLibrary.PrintString` (`KismetStringLibrary.Conv_BoolToString` _returnvalue_2))
      (if _returnvalue_2
        (`StaticMeshComponent.SetStaticMesh` (`self.Obstacle3`) _outitem_2)))
    (:`then_3`
      (`KismetSystemLibrary.PrintString` (`KismetStringLibrary.Conv_BoolToString` _returnvalue_3))
      (if _returnvalue_3
        (`StaticMeshComponent.SetStaticMesh` (`self.Obstacle4`) _outitem)))))

(fn `UserConstructionScript`)